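; PlayerStateTest tracks story progress and the current on-screen text, apparently as a test player state.
; BeginPlay gathers actors attached to "--STORY--"; Step moves an index through them in reverse order, showing each StoryEntry's text for its duration via a rate-scaled timeline.
; ShowDialoge cycles text lines on a looping timer, gating dialogs 11 and 12 behind 10.
; HelpEvents records completed dialogs and reveals an InWorldText after dialog 8.
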(event Custom|ShowDialoge
  (params (Text :type Array%20of%20Strings) (DialogNumber :type Integer) (Time :type Float%20%28single-precision%29) (text_field :type String))
  ;[1 1 1] SpecialCases 11 + 12
  (if (== DialogNumber 11)
    (if (Utilities|Array|ContainsItem (Variables|Default|GetcompletedDialoges) 10)
      (Variables|Default|SetcurrentDialog DialogNumber :!label _label)
      (Variables|Default|SetcurrentText (Utilities|Array|Get(acopy) Text))
      (Math|Integer|IncrementInt (Variables|Default|GetcurrentTextIndex)
        (:%20%20
          (bind _returnvalue (Utilities|Time|SetTimerbyEvent (delegate Custom|HelpEvents) Time true))
          (Variables|Default|SetTimer _returnvalue))))
    (elif (== DialogNumber 12)
      (if (Utilities|Array|ContainsItem (Variables|Default|GetcompletedDialoges) 10)
        (goto _label))
      (else
        (goto _label)))))

(event Custom|StepEvent
  (bind _asstory_entry (Utilities|Casting|CastToStoryEntry (Utilities|Array|Get(acopy) (Variables|Default|GetStoryElements) (- (- (Utilities|Array|Length (Variables|Default|GetStoryElements)) 1) (Variables|Default|Getindex)))))
  (Variables|Default|SetcurrentText (Variables|/Game/Whitebox/Blueprints/GameplayElements/StoryEntry.StoryEntry_C|GetText _asstory_entry))
  (Components|Timeline|SetPlayRate (Variables|Default|GetTimeline_0) (/ 1.0 (Variables|/Game/Whitebox/Blueprints/GameplayElements/StoryEntry.StoryEntry_C|GetTime _asstory_entry)))
  (Timeline|Timeline_0 PlayFromStart
    (:Finished
      (Variables|Default|SetcurrentText ""))))

(event Custom|HelpEvents
  (if (> (Variables|Default|GetcurrentTextIndex) (Utilities|Array|Length (stale Custom|ShowDialoge Text)))
    (Utilities|Array|Add (Variables|Default|GetcompletedDialoges) (stale Custom|ShowDialoge DialogNumber))
    (Variables|Default|SetcurrentTextIndex 0)
    (Variables|Default|SetcurrentText "")
    (Utilities|Time|PauseTimerbyHandle (Variables|Default|GetTimer))
    (if (== (Variables|Default|GetcurrentDialog) 8)
      (bind _actor (Utilities|GetActorbyName (stale Custom|ShowDialoge text_field))
        (:End
          (bind _asin_world_text (Utilities|Casting|CastToInWorldText _actor))
          (Default|ShowText _asin_world_text))))
    (Variables|Default|SetcurrentDialog 0)
    (else
      (Variables|Default|SetcurrentText (Utilities|Array|Get(acopy) (stale Custom|ShowDialoge Text) (Variables|Default|GetcurrentTextIndex)))
      (Math|Integer|IncrementInt (Variables|Default|GetcurrentTextIndex)))))

(event EventBeginPlay
  (bind _actor (Utilities|GetActorbyName "--STORY--")
    (:End
      (bind _output_get (Variables|Default|SetStoryElements (Actor|GetAttachedActors _actor true)))
      (for _array_element _output_get
        _))))

(fn ConstructionScript)

(fn Step
  (params (Calling%20Actor :type Actor%20Object%20Reference) (New%20Current%20State :type String) (Forward :type Boolean))
  (Variables|Default|SetlastAccess Calling%20Actor)
  (if (Utilities|Array|IsEmpty New%20Current%20State)
    _
    (else
      (Variables|Default|SetcurrentState New%20Current%20State)))
  (if Forward
    (Math|Integer|IncrementInt (Variables|Default|Getindex)
      (:%20%20
        _))
    (else
      (Math|Integer|DecrementInt (Variables|Default|Getindex)
        (:%20%20
          _))))
  (CallFunction|StepEvent))