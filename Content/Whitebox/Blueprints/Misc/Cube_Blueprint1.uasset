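; Whitebox cube actor that sets its own yaw from the player's viewing angle onto a passed-in actor, noted as a screen.
; GetActorByName traces from the player, at that actor's height, to the actor on one object channel.
; Yaw is 180 minus the angle between trace direction and hit normal, negated unless the player's Y is lower.
; Unused debug-string and screen-name nodes remain in the graph.
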(fn ConstructionScript)