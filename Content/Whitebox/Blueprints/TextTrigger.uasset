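; TextTrigger is a trigger actor that reveals a piece of in-world text when the player overlaps it.
; On BeginPlay it finds its text actor by name, joining "TF" with three characters taken from index 2 of its own display name, so pairing depends on naming.
; On player overlap it calls ShowText on that InWorldText, first checking FirstPersonCharacter for ItemRequired if one is set.
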(event Collision|EventActorBeginOverlap
  (params (OtherActor :type Actor%20Object%20Reference))
  (bind _returnvalue (Game|Player|GetPlayerPawn 0))
  (bind _item_required (Variables|Default|Getitem_required))
  (if (== OtherActor _returnvalue)
    (bind _asin_world_text (Utilities|Casting|CastToInWorldText (Variables|Default|GetTextActor)))
    (bind _asfirst_person_character (Utilities|Casting|CastToFirstPersonCharacter _returnvalue))
    (if (Utilities|Enum|Equal(Enum) _item_required "")
      (Default|ShowText _asin_world_text :!label _label)
      (else
        (bind _found (Default|CheckforItem _asfirst_person_character _item_required))
        (if _found
          (goto _label))))))

(event EventBeginPlay
  (bind _actor (Utilities|GetActorbyName (Utilities|String|Append "TF" (Utilities|String|GetSubstring (Utilities|GetDisplayName self) 2 3)))
    (:End
      (Variables|Default|SetTextActor _actor))))

(fn ConstructionScript)