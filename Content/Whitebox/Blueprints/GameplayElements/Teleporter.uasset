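; Whitebox teleporter actor that moves any overlapping actor to a matching target location, preserving its offset from the teleporter.
; On BeginPlay it builds the target's name from "TpTarget" plus three characters of its own display name, then caches that actor's location as Goal.
; The lookup scans all actors by display name, so pairing depends on naming rather than references.
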(event EventBeginPlay
  ;[1 1 1] Find respective teleporting target by name
  (bind _actor (Utilities|GetActorbyName (Utilities|String|Append "TpTarget" (Utilities|String|GetSubstring (Utilities|GetDisplayName self) 2 3)))
    (:End
      (Variables|Default|Setgoal (Transformation|GetActorLocation _actor)))))

(event Collision|EventActorBeginOverlap
  (params (OtherActor :type Actor%20Object%20Reference))
  (bind _returnvalue (Transformation|GetActorLocation OtherActor))
  (bind _self self)
  (bind _goal (Variables|Default|Getgoal))
  (bind _returnvalue_2 (Transformation|GetActorLocation _self))
  (bind _returnvalue_3 (- _returnvalue _returnvalue_2))
  (bind _returnvalue_4 (+ _returnvalue_3 _goal))
  (bind (_x _y _z) (Math|Vector|BreakVector _returnvalue_4))
  ;[1 1 1] Teleport player to respective target
  (Transformation|SetActorLocation OtherActor (Math|Vector|MakeVector _x _y _z) false true))

(fn ConstructionScript)

(fn GetActorbyName1
  (params (ActorName :type String))
  (bind _outactors (Actor|GetAllActorsOfClass "/Script/Engine.Actor"))
  (for _array_element _outactors
    (if (Utilities|Enum|Equal(Enum) (Utilities|GetDisplayName _array_element) ActorName)
      (return _array_element)))
  (return 0))