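; A one-shot trigger box that advances the player's progression state when a player-controlled actor overlaps it.
; On overlap, it optionally requires a minimum PlayerStateTest index, then marks itself used and calls Step forward.
; When an item requirement is set, it calls CheckForItem on the FirstPersonCharacter first, but continues to the index check without reading a result.
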(event Collision|EventActorBeginOverlap
  (params (OtherActor :type Actor%20Object%20Reference))
  (if (and (Pawn|IsPlayerControlled (Variables|/Script/Engine.Actor|GetInstigator OtherActor)) (not (Variables|Default|Getused)))
    (if (Utilities|Array|IsEmpty (Variables|Default|Getitem_requirement))
      _
      (else
        (bind _asfirst_person_character (Utilities|Casting|CastToFirstPersonCharacter (Game|Player|GetPlayerPawn 0)))
        (Default|CheckforItem _asfirst_person_character (Variables|Default|Getitem_requirement))))
    (bind _asplayer_state_test (Utilities|Casting|CastToPlayerStateTest (Variables|/Script/Engine.Pawn|GetPlayerState (Game|Player|GetPlayerPawn 0))))
    (if (== (Variables|Default|Getindex_requirement) 0)
      (Variables|Default|Setused true :!label _label)
      (Default|Step _asplayer_state_test self "" true)
      (elif (>= (Variables|/Game/Whitebox/Blueprints/Misc/PlayerStateTest.PlayerStateTest_C|Getindex _asplayer_state_test) (Variables|Default|Getindex_requirement))
        (goto _label)))))

(fn ConstructionScript)