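; Keypad actor in which the player types a four-character combination on the keyboard, with click, accept and deny sounds.
; EnterCode blocks character input and enables the keypad's own, comparing each key's display name to the next Combination character.
; A wrong key zeroes the index but leaves the expected character unchanged.
; Completion prints a message, restores character input and calls EndKeyPad on the character.
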(event Custom|EnterCode
  ;[1 1 1] Entering
  (Variables|Default|Setactive true)
  (bind _asfirst_person_character (Utilities|Casting|CastToFirstPersonCharacter (Game|Player|GetPlayerPawn 0)))
  (Variables|/Game/Whitebox/PlayerCharacter/FirstPersonCharacter.FirstPersonCharacter_C|SetinputAllowed _asfirst_person_character false)
  (Variables|Default|SetneededKey (Utilities|String|GetSubstring (Variables|Default|Getcombination) 0))
  (Input|EnableInput (Game|GetPlayerController 0)))

(event Custom|WrongKey
  ;[1 1 1] Wrong Key
  (Variables|Default|Setindex 0)
  (Utilities|FlowControl|Delay 0.1)
  (Audio|PlaySoundatLocation "/Game/Whitebox/Blueprints/GameplayElements/KeyPadTesting/denie.denie" (Transformation|GetActorLocation self) "0, 0, 0" 1.0 1.0 0.0 0 0 0))

(event Custom|CorrectComb
  ;[1 1 1] Correct Combination
  (Variables|Default|Setactive false)
  (Development|PrintString "Correct!")
  (bind _asfirst_person_character (Utilities|Casting|CastToFirstPersonCharacter (Game|Player|GetPlayerPawn 0)))
  (Variables|/Game/Whitebox/PlayerCharacter/FirstPersonCharacter.FirstPersonCharacter_C|SetinputAllowed _asfirst_person_character true)
  (Input|DisableInput (Game|GetPlayerController 0))
  (Default|EndKeyPad _asfirst_person_character)
  (Variables|Default|Setindex 0)
  (Utilities|FlowControl|Delay 0.1)
  (Audio|PlaySoundatLocation "/Game/Whitebox/Blueprints/GameplayElements/KeyPadTesting/accepted.accepted" (Transformation|GetActorLocation self) "0, 0, 0" 1.0 1.0 0.0 0 0 0))

(event Custom|CorrectKey)

(event EventBeginPlay
  (Input|DisableInput (Game|GetPlayerController 0)))

(event Input|KeyboardEvents|AnyKey
  (params (Key :type Key%20Structure))
  ;[1 1 1] Handling input
  (:Pressed
    (if (Variables|Default|Getactive)
      (Audio|PlaySoundatLocation "/Game/Whitebox/Blueprints/GameplayElements/KeyPadTesting/click.click" (Transformation|GetActorLocation self) "0, 0, 0" 1.0 1.0 0.0 0 0 0)
      (if (Utilities|Enum|Equal(Enum) (Utilities|String|ToString(Text) (Class|KismetInputLibrary|KeyGetDisplayName Key)) (Variables|Default|GetneededKey))
        (bind _result (Math|Integer|IncrementInt (Variables|Default|Getindex))
          (:%20%20
            (CallFunction|CorrectKey)
            (if (== (Variables|Default|Getindex) 4)
              (CallFunction|CorrectComb)
              (else
                (Variables|Default|SetneededKey (Utilities|String|GetSubstring (Variables|Default|Getcombination) _result))))))
        (else
          (CallFunction|WrongKey))))))

(fn ConstructionScript)