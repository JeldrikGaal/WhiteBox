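; Whitebox dialog trigger actor that shows story conversations between THIEF and ANA when an overlap begins.
; BeginPlay fills DialogList with hardcoded dialog objects, each holding text lines, a dialog number and a time.
; On overlap, entries matching this actor's Dialognum are passed to ShowDialoge on player 0's PlayerStateTest.
; The overlapping actor is not checked, and the trigger has no once-only guard.
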(event EventBeginPlay
  (Utilities|Array|Add (Variables|Default|GetdialogList) (Utilities|Struct|Makedialog_object (Utilities|Array|MakeArray "THIEF 
It’s locked. " "ANA 
Wow. Some master thief you are, deterred by a single lock. " "THIEF 
No need to get snarky, I’ll have a look around and see if I can 
find the code. ") 3 2.0))
  (Utilities|Array|Add (Variables|Default|GetdialogList) (Utilities|Struct|Makedialog_object (Utilities|Array|MakeArray "THIEF 
The lights are on. " "ANA 
So we can add energy waster to our profile of Marsden. " "THIEF 
You’re sure the house is empty? " "ANA 
Yes. He lives alone and he already left. ") 4 2.0))
  (Utilities|Array|Add (Variables|Default|GetdialogList) (Utilities|Struct|Makedialog_object (Utilities|Array|MakeArray "ANA 
What are you doing? " "THIEF 
I am not snooping. I am looking for the rest of the code. " "ANA 
You think he wrote it down twice? " "THIEF 
Just a hunch. ") 5 2.0))
  (Utilities|Array|Add (Variables|Default|GetdialogList) (Utilities|Struct|Makedialog_object (Utilities|Array|MakeArray "THIEF 
Are you sure we are in the right house? These look like a 
child drew them. Not a world famous painter. " "ANA 
Guess thats why he threw them away. ") 6 2.0))
  (Utilities|Array|Add (Variables|Default|GetdialogList) (Utilities|Struct|Makedialog_object (Utilities|Array|MakeArray "THIEF 
You said that Emil Marsden just finished this glorious piece of 
art — yet he doesn’t seem to be in any condition to even feed 
himself. " "ANA 
It is strange, yes. But my sources are reliable. " "THIEF 
Convenient. ") 7 2.0))
  (Utilities|Array|Add (Variables|Default|GetdialogList) (Utilities|Struct|Makedialog_object (Utilities|Array|MakeArray "THIEF 
Emil was loosing his eye sight after the accident. Why else would 
he need this? This whole house-… Ana - I don’t think he is 
painting anymore. " "ANA 
Yes he is. He has to be. Without his art, my brother beliefs he is 
nothing. ") 10 2.0))
  (Utilities|Array|Add (Variables|Default|GetdialogList) (Utilities|Struct|Makedialog_object (Utilities|Array|MakeArray "ANA 
Listen. You have to find this painting. It is vital. " "THIEF 
How? I need the whole code. " "ANA 
Use the braille signs. You need them. ") 11 2.0))
  (Utilities|Array|Add (Variables|Default|GetdialogList) (Utilities|Struct|Makedialog_object (Utilities|Array|MakeArray "ANA 
I know I haven’t been completely honest with you. But I need you 
to focus. I need to find this painting. Without it, my brother is 
lost. For him his art and his success means everything. If we 
can’t find it, Emil will be gone as well.") 12 2.0)))

(event Collision|EventActorBeginOverlap
  (params (OtherActor :type Actor%20Object%20Reference))
  (for _array_element (Variables|Default|GetdialogList)
    (if (== (.dialog_number (Utilities|Struct|Breakdialog_object _array_element)) (Variables|Default|Getdialognum))
      (bind _asplayer_state_test (Utilities|Casting|CastToPlayerStateTest (Variables|/Script/Engine.Pawn|GetPlayerState (Game|Player|GetPlayerPawn 0))))
      (Default|ShowDialoge _asplayer_state_test (.text (Utilities|Struct|Breakdialog_object _array_element)) (.dialog_number (Utilities|Struct|Breakdialog_object _array_element)) (.time (Utilities|Struct|Breakdialog_object _array_element))))))

(fn ConstructionScript)