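; Whitebox trigger actor that turns the player's view around when an actor overlaps it.
; On overlap it adds 180 degrees to the first player controller's yaw, keeping pitch and roll.
; It then teleports itself to the overlapping actor's Y and Z, with X set by reflecting that actor's X across its own.
; A DoOnce gate, reset after a one-second delay, blocks immediate retriggering.
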(event Collision|EventActorBeginOverlap
  (params (OtherActor :type Actor%20Object%20Reference))
  (bind _returnvalue (Game|GetPlayerController 0))
  (bind _returnvalue_2 (Transformation|GetActorLocation OtherActor))
  (bind _returnvalue_3 (Transformation|GetActorLocation))
  (bind _returnvalue_4 (Pawn|GetControlRotation _returnvalue :!class /Script/Engine.Controller))
  ;[1 1 1] Turn
  (Utilities|FlowControl|DoOnce false :!label _label
    (:Completed
      (Pawn|SetControlRotation _returnvalue (Math|Rotator|MakeRotator (.roll _returnvalue_4) (.pitch _returnvalue_4) (+ (.yaw _returnvalue_4) 1.8e+02)))
      (Transformation|SetActorLocation (Math|Vector|MakeVector (+ (.x _returnvalue_3) (- (.x _returnvalue_3) (.x _returnvalue_2))) (.y _returnvalue_2) (.z _returnvalue_2)) false true)
      (Utilities|FlowControl|Delay 1.0)
      (goto _label Reset))))

(fn ConstructionScript)