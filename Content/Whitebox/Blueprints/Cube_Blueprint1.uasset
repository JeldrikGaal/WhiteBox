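; Whitebox cube actor that sets its own yaw from the angle between the player and a given actor, noted as a screen.
; Its GetActorByName event traces from the player's XY, at that actor's height, to the actor.
; The dot product of trace direction and hit normal gives the yaw, negated unless the player's Y is lower than the actor's.
; Debug-string and screen-name nodes are unused.
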(fn ConstructionScript)